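; BP_Item is a collectible pickup that the player collects with the IA_PickUp input while standing in its collision.
; Overlap begin and end with BP_ThirdPersonCharacter toggle the actor's input, so only nearby items respond to the key.
; On pickup it decrements the character's Remaining count, shows a WB_Collected widget and destroys itself.
; When Remaining reaches zero it quits the game.
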(event `EnhancedInput|/Game/ThirdPerson/Input/Actions/IA_PickUp`
  (params (ActionValue :type Boolean) (ElapsedSeconds :type "Float (double-precision)") (TriggeredSeconds :type "Float (double-precision)") (InputAction :type "InputAction Object Reference" :default "/Game/ThirdPerson/Input/Actions/IA_PickUp.IA_PickUp"))
  (:`Started`
    (bind _asbp_third_person_character (cast `/Game/ThirdPerson/Blueprints/BP_ThirdPersonCharacter` (`GameplayStatics.GetPlayerCharacter` 0)))
    (bind _result (`/Engine/EditorBlueprintResources/StandardMacros.DecrementInt` (`/Game/ThirdPerson/Blueprints/BP_ThirdPersonCharacter.Remaining` _asbp_third_person_character))
      (:`  `
        (set `/Game/ThirdPerson/Blueprints/BP_ThirdPersonCharacter.Remaining` _result _asbp_third_person_character)
        (bind _returnvalue (`|CreateWidget` "/Game/Items/WB_Collected.WB_Collected_C"))
        (`UserWidget.AddToViewport` _returnvalue 0)
        (`self.K2_DestroyActor`)
        (if (== (`/Game/ThirdPerson/Blueprints/BP_ThirdPersonCharacter.Remaining` _asbp_third_person_character) 0)
          (`KismetSystemLibrary.QuitGame` null "Quit"))))))

(event `self.Collision.OnComponentBeginOverlap`
  (params (OverlappedComponent :type "PrimitiveComponent Object Reference") (OtherActor :type "Actor Object Reference") (OtherComp :type "PrimitiveComponent Object Reference") (OtherBodyIndex :type Integer) (bFromSweep :type Boolean) (SweepResult :type "HitResult Structure (by ref)"))
  (cast `/Game/ThirdPerson/Blueprints/BP_ThirdPersonCharacter` OtherActor)
  (`self.EnableInput` (`GameplayStatics.GetPlayerController` 0)))

(event `self.Collision.OnComponentEndOverlap`
  (params (OverlappedComponent :type "PrimitiveComponent Object Reference") (OtherActor :type "Actor Object Reference") (OtherComp :type "PrimitiveComponent Object Reference") (OtherBodyIndex :type Integer))
  (cast `/Game/ThirdPerson/Blueprints/BP_ThirdPersonCharacter` OtherActor)
  (`self.DisableInput` (`GameplayStatics.GetPlayerController` 0)))

(fn `UserConstructionScript`)